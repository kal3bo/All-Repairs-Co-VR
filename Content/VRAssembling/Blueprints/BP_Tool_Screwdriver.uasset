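; BP_Tool_Screwdriver is a VR assembly tool that drives screwable parts while its trigger is held, with a spotlight visible meanwhile.
; Face button 1 flips the screwing direction and rotates a mesh half a turn, while face button 2 cycles head types and their meshes.
; On Tick, screwable parts overlapping the tip sphere that pass a forward-vector alignment test receive Screw with the head name and frame-scaled speed.
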(event `/Game/VRAssembling/Blueprints/BI_Input.TriggerPress`
  (bind _output_get (set `self.Screwing` true))
  (`SceneComponent.SetVisibility` (`self.SpotLight`) _output_get false :!label _label))

(event `/Game/VRAssembling/Blueprints/BI_Input.TriggerRelease`
  (set `self.Screwing` false)
  (goto _label))

(event `/Game/VRAssembling/Blueprints/BI_Input.FaceButton1Release`
  (set `self.Speed` (* (`self.Speed`) -1.0))
  (`SceneComponent.K2_AddRelativeRotation` (`self.StaticMesh1`) (struct :`Yaw` 180.0) false false))

(event `/Game/VRAssembling/Blueprints/BI_Input.FaceButton2Release`
  (set `self.Head` (mod (+ (`self.Head`) 1) (`KismetArrayLibrary.Array_Length` (`self.HeadNames`))))
  (`self.SetHeadMesh`))

(event `SetHeadMesh`
  (if true
    (`StaticMeshComponent.SetStaticMesh` (`self.HeadMesh`) (`|GetArrayItem` (`self.Heads`) (`self.Head`)))))

(event `self.ReceiveTick`
  (params (DeltaSeconds :type "Float (single-precision)"))
  (if (`self.Screwing`)
    (for _array_element (`PrimitiveComponent.GetOverlappingActors` (`self.Sphere`) null)
      (bind _asbp_part_screwable (cast `/Game/VRAssembling/Blueprints/BP_Part_Screwable` _array_element))
      (if (> (`KismetMathLibrary.Dot_VectorVector` (`SceneComponent.GetForwardVector` (`self.Sphere`)) (`self.GetActorForwardVector` _asbp_part_screwable)) (`self.ScrewableFaceMargin`))
        (`/Game/VRAssembling/Blueprints/BP_Part_Screwable.Screw` _asbp_part_screwable (`|GetArrayItem` (`self.HeadNames`) (`self.Head`)) (* (`self.Speed`) DeltaSeconds))))))

(fn `UserConstructionScript`
  (`parent.UserConstructionScript`)
  (`self.SetHeadMesh`))